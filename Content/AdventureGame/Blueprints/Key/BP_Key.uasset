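; BP_Key is a collectible key pickup for the adventure game, with a configurable key type.
; Its construction script passes the key mesh, key map and type to FnBPLSetKey to set up the key.
; When an actor implementing BPI_PlayerKeys overlaps the capsule, the key sends its type through that interface, then destroys itself after a short delay.
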(event OnComponentBeginOverlap(Capsule)
  (params (OverlappedComponent :type Primitive%20Component%20Object%20Reference) (OtherActor :type Actor%20Object%20Reference) (OtherComp :type Primitive%20Component%20Object%20Reference) (OtherBodyIndex :type Integer) (bFromSweep :type Boolean) (SweepResult :type Hit%20Result%20Structure%20%28by%20ref%29))
  (bind _output_get (Variables|Default|SetOtherActor OtherActor))
  (if (Utilities|DoesObjectImplementInterface _output_get "/Game/AdventureGame/Blueprints/Key/BPI_PlayerKeys.BPI_PlayerKeys_C")
    (Class|BPIPlayerKeys|FnBPIAddKey(Message) (Variables|Default|GetOtherActor) (Variables|Default|GetKeyType))
    (Utilities|FlowControl|Delay 0.2)
    (Actor|DestroyActor)))

(event EventBeginPlay)

(event Collision|EventActorBeginOverlap
  (params (OtherActor :type Actor%20Object%20Reference)))

(event EventTick
  (params (DeltaSeconds :type Float%20%28single-precision%29)))

(fn ConstructionScript
  (CallFunction|FnBPLSetKey (Utilities|Array|MakeArray (Variables|Default|GetKeyMesh)) (Variables|Default|GetKeyMap) (Variables|Default|GetKeyType)))
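; BP_LevelTransition is a level exit trigger that ends the level when the overlapping actor holds all required keys.
; On LevelTrigger overlap, it gets the actor's held keys through an interface message and checks each RequiredKeys entry, stopping at the first missing one.
; If all are found, it disables the actor's input, shows WBP_WinScreen, then opens NextLevel after a configurable delay.
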(event OnComponentBeginOverlap(LevelTrigger)
  (params (OverlappedComponent :type Primitive%20Component%20Object%20Reference) (OtherActor :type Actor%20Object%20Reference) (OtherComp :type Primitive%20Component%20Object%20Reference) (OtherBodyIndex :type Integer) (bFromSweep :type Boolean) (SweepResult :type Hit%20Result%20Structure%20%28by%20ref%29))
  (Variables|Default|SetOtherActor OtherActor)
  (bind _held_keys (Class|BPIPlayerKeys|FnBPIGetKeys(Message) (Variables|Default|GetOtherActor)))
  (Variables|Default|SetHeldKeys _held_keys)
  (bind _array_element (Utilities|Array|ForEachLoopwithBreak (Variables|Default|GetRequiredKeys) :!label _label)
    (:LoopBody
      (if (Utilities|Array|ContainsItem (Variables|Default|GetHeldKeys) _array_element)
        (Variables|Default|SetFoundAllKeys true)
        (else
          (Variables|Default|SetFoundAllKeys false)
          (goto _label Break))))
    (:Completed
      (if (Variables|Default|GetFoundAllKeys)
        (Utilities|FlowControl|Sequence
          (:then_0
            (Input|DisableInput (Variables|Default|GetOtherActor) (Game|GetPlayerController 0)))
          (:then_1
            (bind _returnvalue (UserInterface|CreateWidget "/Game/AdventureGame/Designer/Blueprints/Widgets/WBP_WinScreen.WBP_WinScreen_C"))
            (UserInterface|Viewport|AddtoViewport _returnvalue 0))
          (:then_2
            (Utilities|FlowControl|Delay (Variables|Default|GetLoadLevelDelay))
            (Game|OpenLevel(byObjectReference) (Variables|Default|GetNextLevel))))))))

(event EventBeginPlay)

(event Collision|EventActorBeginOverlap
  (params (OtherActor :type Actor%20Object%20Reference)))

(event EventTick
  (params (DeltaSeconds :type Float%20%28single-precision%29)))

(fn ConstructionScript)
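; BP_Enemy is an enemy character that chases the player and damages them on capsule contact, destroying itself shortly after.
; Tick runs a shared detection function within a maximum distance, re-issuing AI Move To while the player is found and zeroing walk speed otherwise.
; Move completion or failure retries the chase after a delay.
; Incoming damage reduces HP, and reaching zero marks it eliminated, halting detection before delayed destruction.
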(event OnComponentHit(CapsuleComponent)
  (params (HitComponent :type Primitive%20Component%20Object%20Reference) (OtherActor :type Actor%20Object%20Reference) (OtherComp :type Primitive%20Component%20Object%20Reference) (NormalImpulse :type Vector :default "0, 0, 0") (Hit :type Hit%20Result%20Structure%20%28by%20ref%29))
  (bind _playerref (Variables|Default|GetPlayerRef))
  (if (== OtherActor _playerref)
    (Utilities|FlowControl|DoOnce false
      (:Completed
        (Game|Damage|ApplyDamage _playerref (Variables|Setup|GetBase%20Damage) 0 0)
        (Variables|Default|SetEliminated true)
        (Utilities|FlowControl|Delay 0.2)
        (Actor|DestroyActor)))))

(event Custom|MoveToPlayer
  (if (Variables|Default|GetFound)
    (AI|AIMoveTo self "0, 0, 0" (Variables|Default|GetPlayerRef) 1e+01 false
      (:OnSuccess
        (Utilities|FlowControl|Delay (Variables|Setup|GetWaitAtDestination))
        (CallFunction|MovetoPlayer))
      (:OnFail
        (Utilities|FlowControl|Delay 0.2)
        (CallFunction|MovetoPlayer)))))

(event EventBeginPlay
  (Variables|/Script/Engine.CharacterMovementComponent|SetMaxWalkSpeed (Variables|Character|GetCharacterMovement) (Variables|Setup|GetMax%20Speed))
  (Variables|Default|SetCurrentHP (Variables|Setup|GetTotalHP))
  (Variables|Default|SetPlayerRef (Game|GetPlayerCharacter 0))
  (CallFunction|MovetoPlayer))

(event EventTick
  (params (DeltaSeconds :type Float%20%28single-precision%29))
  (if (not (Variables|Default|GetEliminated))
    (bind _found (CallFunction|FnBPLFindPlayer (Variables|Default|GetPlayerRef) (Transformation|GetActorLocation) (Variables|Setup|GetMax%20Detection%20Distance) (Variables|Setup|GetDebugDetection)))
    (bind _output_get (Variables|Default|SetFound _found))
    (if _output_get
      (Variables|/Script/Engine.CharacterMovementComponent|SetMaxWalkSpeed (Variables|Character|GetCharacterMovement) (Variables|Setup|GetMax%20Speed))
      (CallFunction|MovetoPlayer)
      (else
        (Variables|/Script/Engine.CharacterMovementComponent|SetMaxWalkSpeed (Variables|Character|GetCharacterMovement) 0.0)))))

(event Game|Damage|EventAnyDamage
  (params (Damage :type Float%20%28single-precision%29) (DamageType :type Damage%20Type%20Object%20Reference) (InstigatedBy :type Controller%20Object%20Reference) (DamageCauser :type Actor%20Object%20Reference))
  (bind _output_get (Variables|Default|SetCurrentHP (- (Variables|Default|GetCurrentHP) Damage)))
  (if (<= _output_get 0.0)
    (Utilities|FlowControl|DoOnce false
      (:Completed
        (Variables|Default|SetEliminated true)
        (Utilities|FlowControl|Delay 2.0)
        (Actor|DestroyActor)))))

(fn ConstructionScript)
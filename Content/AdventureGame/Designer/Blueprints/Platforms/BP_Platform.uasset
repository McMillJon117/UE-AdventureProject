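; BP_Platform is a switchable moving platform that shuttles between its starting location and a TargetPoint actor.
; A timeline lerps the Platform component's position and, while Active, reverses after a delay at each end.
; Interface-style switch events toggle Active; switching off lets the current leg finish.
; TimeToTarget feeds the timeline's play rate directly, so larger values move faster, and the construction script applies PlatformScale.
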(event Custom|Stop
  (bind (_direction _alpha) (Timeline|MovePlatform Stop)
    (:Update
      (Transformation|SetWorldLocation (Variables|Default|GetPlatform) (Math|Vector|Lerp(Vector) (Variables|Default|GetStartLocation) (Variables|Default|GetEndLocation) _alpha) false false))
    (:Finished
      (Utilities|FlowControl|Delay (Variables|Default|GetWaitDuration))
      (if (Variables|Default|GetActive)
        (if (Utilities|Enum|Equal(Enum) _direction "Forward")
          (CallFunction|MoveBackward)
          (else
            (CallFunction|MoveForward)))))))

(event Custom|MoveForward
  (bind (_direction _alpha) (Timeline|MovePlatform Play)
    (:Update
      (Transformation|SetWorldLocation (Variables|Default|GetPlatform) (Math|Vector|Lerp(Vector) (Variables|Default|GetStartLocation) (Variables|Default|GetEndLocation) _alpha) false false))
    (:Finished
      (Utilities|FlowControl|Delay (Variables|Default|GetWaitDuration))
      (if (Variables|Default|GetActive)
        (if (Utilities|Enum|Equal(Enum) _direction "Forward")
          (CallFunction|MoveBackward)
          (else
            (CallFunction|MoveForward)))))))

(event Custom|MoveBackward
  (bind (_direction _alpha) (Timeline|MovePlatform Reverse)
    (:Update
      (Transformation|SetWorldLocation (Variables|Default|GetPlatform) (Math|Vector|Lerp(Vector) (Variables|Default|GetStartLocation) (Variables|Default|GetEndLocation) _alpha) false false))
    (:Finished
      (Utilities|FlowControl|Delay (Variables|Default|GetWaitDuration))
      (if (Variables|Default|GetActive)
        (if (Utilities|Enum|Equal(Enum) _direction "Forward")
          (CallFunction|MoveBackward)
          (else
            (CallFunction|MoveForward)))))))

(event EventBeginPlay
  (Variables|Default|SetStartLocation (Transformation|GetActorLocation))
  (Variables|Default|SetEndLocation (Transformation|GetActorLocation (Variables|Default|GetTargetPoint)))
  (Components|Timeline|SetPlayRate (Variables|Default|GetMovePlatform) (Variables|Default|GetTimeToTarget))
  (if (Variables|Default|GetActive)
    (CallFunction|MoveForward)))

(event EventFnBPISwitchon
  (Variables|Default|SetActive true)
  (CallFunction|MoveForward))

(event EventFnBPISwitchOff
  (Variables|Default|SetActive false))

(fn ConstructionScript
  (Transformation|SetWorldScale3D (Variables|Default|GetPlatform) (Variables|Default|GetPlatformScale)))
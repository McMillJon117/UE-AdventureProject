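; Overlap-activated switch actor that turns a list of linked objects on and off.
; Entering the Trigger applies the on material and sends a switch-on interface message to each object in InteractObjectList, repeating on every new overlap.
; Unless ActivateOnce is set, it reverts the material and sends switch-off messages once no actors remain in the Trigger.
; The construction script starts the switch with the off material.
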(event OnComponentBeginOverlap(Trigger)
  (params (OverlappedComponent :type Primitive%20Component%20Object%20Reference) (OtherActor :type Actor%20Object%20Reference) (OtherComp :type Primitive%20Component%20Object%20Reference) (OtherBodyIndex :type Integer) (bFromSweep :type Boolean) (SweepResult :type Hit%20Result%20Structure%20%28by%20ref%29))
  (Rendering|Material|SetMaterial (Variables|Default|GetSwitch) 0 (Variables|Default|GetOnMaterial))
  (for _array_element (Variables|Default|GetInteractObjectList)
    (Class|BPIInteraction|FnBPISwitchon(Message) _array_element)))

(event OnComponentEndOverlap(Trigger)
  (params (OverlappedComponent :type Primitive%20Component%20Object%20Reference) (OtherActor :type Actor%20Object%20Reference) (OtherComp :type Primitive%20Component%20Object%20Reference) (OtherBodyIndex :type Integer))
  (if (not (Variables|Default|GetActivateOnce))
    (if (Utilities|Array|IsEmpty (Collision|GetOverlappingActors (Variables|Default|GetTrigger) "/Script/Engine.Actor" :!class /Script/Engine.PrimitiveComponent))
      (Rendering|Material|SetMaterial (Variables|Default|GetSwitch) 0 (Variables|Default|GetOffMaterial))
      (for _array_element (Variables|Default|GetInteractObjectList)
        (Class|BPIInteraction|FnBPISwitchOff(Message) _array_element)))))

(event EventBeginPlay)

(event Collision|EventActorBeginOverlap
  (params (OtherActor :type Actor%20Object%20Reference)))

(event EventTick
  (params (DeltaSeconds :type Float%20%28single-precision%29)))

(fn ConstructionScript
  (Rendering|Material|SetMaterial (Variables|Default|GetSwitch) 0 (Variables|Default|GetOffMaterial)))
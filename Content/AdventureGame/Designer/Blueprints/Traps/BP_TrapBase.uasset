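; BP_TrapBase is a trap Blueprint that damages Characters inside its TrapTrigger volume while Active.
; If Active at BeginPlay, it creates a paused looping timer on DamageInterval.
; Overlap begin applies damage immediately and unpauses the timer; any overlap end pauses it, even if others remain inside.
; Each damage pass hits every overlapping Character with BaseDamage and prints a debug message.
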(event OnComponentBeginOverlap(TrapTrigger)
  (params (OverlappedComponent :type Primitive%20Component%20Object%20Reference) (OtherActor :type Actor%20Object%20Reference) (OtherComp :type Primitive%20Component%20Object%20Reference) (OtherBodyIndex :type Integer) (bFromSweep :type Boolean) (SweepResult :type Hit%20Result%20Structure%20%28by%20ref%29))
  (Variables|Default|SetOtherActor OtherActor)
  (CallFunction|FnApplyDamagetoTarget)
  (Utilities|Time|UnpauseTimerbyHandle (Variables|Default|GetTimerHandler)))

(event OnComponentEndOverlap(TrapTrigger)
  (params (OverlappedComponent :type Primitive%20Component%20Object%20Reference) (OtherActor :type Actor%20Object%20Reference) (OtherComp :type Primitive%20Component%20Object%20Reference) (OtherBodyIndex :type Integer))
  (Utilities|Time|PauseTimerbyHandle (Variables|Default|GetTimerHandler)))

(event EventBeginPlay
  (if (Variables|Setup|GetActive)
    (bind _returnvalue (Utilities|Time|SetTimerbyFunctionName 0 "fnApplyDamageToTarget" (Variables|Setup|GetDamageInterval) true))
    (bind _output_get (Variables|Default|SetTimerHandler _returnvalue))
    (Utilities|Time|PauseTimerbyHandle _output_get)))

(fn ConstructionScript)

(fn FnApplyDamagetoTarget
  (if (Variables|Setup|GetActive)
    (for _array_element (Collision|GetOverlappingActors (Variables|Default|GetTrapTrigger) "/Script/Engine.Character" :!class /Script/Engine.PrimitiveComponent)
      (Game|Damage|ApplyDamage _array_element (Variables|Setup|GetBaseDamage) 0 0)
      (Development|PrintString "Player Hit"))))